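; BP_InteractiveActor is an interactive actor that accepts player input only while the player character overlaps it.
; On BeginPlay it casts the player pawn to BP_ThirdPersonCharacter and caches it as Player.
; Overlap begin and end events check for that character, then enable or disable input from the first player controller.
; The graph defines no input actions or interaction response of its own.
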(event `self.ReceiveBeginPlay`
  ;[0.05061 0.15 0.03039 0.5] Beginplay
  (bind _asbp_third_person_character (cast `/Game/ThirdPerson/Blueprints/BP_ThirdPersonCharacter` (`GameplayStatics.GetPlayerPawn` 0)))
  (set `self.Player` _asbp_third_person_character))

(event `self.ReceiveActorBeginOverlap`
  (params (OtherActor :type "Actor Object Reference"))
  ;[0.15 0.1304 0.03356 0.5] BeginOverlap
  (if (== OtherActor (`self.Player`))
    (`self.EnableInput` (`GameplayStatics.GetPlayerController` 0))))

(event `self.ReceiveActorEndOverlap`
  (params (OtherActor :type "Actor Object Reference"))
  ;[0.15 0.007734 0.006242 0.5] EndOverlap
  (if (== OtherActor (`self.Player`))
    (`self.DisableInput` (`GameplayStatics.GetPlayerController` 0))))

(fn `UserConstructionScript`)